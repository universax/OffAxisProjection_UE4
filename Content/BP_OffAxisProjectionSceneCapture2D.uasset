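; Scene capture actor that renders an off-axis projection through a BP_OffAxisProjectionTargetScreen, treating the screen as the projection window.
; Each Tick, it feeds three screen corner points to SetTargetQuadPoints to update the projection matrix, then matches its rotation to the screen's.
; An optional debug toggle draws colored lines from the capture to those corners.
; The construction script hides all target screen actors from the capture.
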(event EventBeginPlay)

(event EventTick
  (params (DeltaSeconds :type Float%20%28single-precision%29))
  (bind _returnvalue (Transformation|GetActorLocation))
  (bind _offaxisprojection_targetscreen (Variables|Default|GetOffAxisProjection_TargetScreen))
  (Utilities|IsValid _offaxisprojection_targetscreen
    (:Is%20Valid
      (Utilities|FlowControl|Sequence
        (:then_0
          ;[1 1 1] Get Screen Edge Verts Location
          (bind (_pa _pb _pc) (Default|GetCornerPoints _offaxisprojection_targetscreen))
          (Variables|Default|SetPa _pa)
          (Variables|Default|SetPb _pb)
          (Variables|Default|SetPc _pc)
          ;[1 1 1] Update Projection Matrix
          (Class|OffAxisProjectionSceneCapture2D|SetTargetQuadPoints (Variables|Default|GetPa) (Variables|Default|GetPb) (Variables|Default|GetPc))
          ;[1 1 1] Debug Ray
          (if (Variables|Default|GetEnableDebugRay)
            (Utilities|FlowControl|Sequence
              (:then_0
                (Rendering|Debug|DrawDebugLine _returnvalue (Variables|Default|GetPa) "(R=1.000000,G=0.000000,B=0.000000,A=1.000000)" 0.0 1.0))
              (:then_1
                (Rendering|Debug|DrawDebugLine _returnvalue (Variables|Default|GetPb) "(R=0.000000,G=1.000000,B=0.000000,A=1.000000)" 0.0 1.0))
              (:then_2
                (Rendering|Debug|DrawDebugLine _returnvalue (Variables|Default|GetPc) "(R=0.000000,G=1.000000,B=1.000000,A=1.000000)" 0.0 1.0)))))
        (:then_1
          ;[1 1 1] Set Cam Rot from Screen Rot
          (Transformation|SetActorRotation (Transformation|GetActorRotation _offaxisprojection_targetscreen)))))))

(fn ConstructionScript
  (bind _outactors (Actor|GetAllActorsOfClass "/OffAxisProjection/BP_OffAxisProjectionTargetScreen.BP_OffAxisProjectionTargetScreen_C"))
  (Variables|/Script/Engine.SceneCaptureComponent|SetHiddenActors (Variables|Default|GetCaptureComponent2D) _outactors))