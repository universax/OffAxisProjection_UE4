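; Screen actor that marks a target rectangle for off-axis projection by exposing three of its corners.
; Its construction script offsets bottom-left, bottom-right and top-left markers by half the ScreenGuide's scaled 100-unit Y/Z size, divided by guide scale for local space.
; GetCornerPoints returns their world positions as Pa, Pb and Pc.
; It has no runtime event logic.
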(event EventBeginPlay)

(event Collision|EventActorBeginOverlap
  (params (OtherActor :type Actor%20Object%20Reference)))

(event EventTick
  (params (DeltaSeconds :type Float%20%28single-precision%29)))

(fn ConstructionScript
  (CallFunction|UpdateCornerWorldPositions))

(fn UpdateCornerWorldPositions
  (bind _lb_pa (Variables|Default|GetLB_pa))
  (bind _rb_pb (Variables|Default|GetRB_pb))
  (bind _lt_pc (Variables|Default|GetLT_pc))
  (bind _screenguide (Variables|Default|GetScreenGuide))
  (bind _returnvalue (Transformation|GetWorldScale _screenguide))
  (bind _returnvalue_2 (* _returnvalue 1e+02))
  (bind _returnvalue_3 (* _returnvalue_2 0.5))
  (bind (_x _y _z) (Math|Vector|BreakVector _returnvalue_3))
  (bind (_x_2 _y_2 _z_2) (Math|Vector|BreakVector _returnvalue_3))
  (bind (_x_3 _y_3 _z_3) (Math|Vector|BreakVector _returnvalue_3))
  (LocalVariables|SetRootOffset (Transformation|GetWorldLocation _screenguide))
  (Utilities|FlowControl|Sequence
    (:then_0
      (Transformation|SetWorldScale3D _lb_pa "0.100000,0.100000,0.100000")
      (Transformation|AddLocalOffset _lb_pa (/ (Math|Vector|MakeVector 0.0 (* _y -1.0) (* _z -1.0)) (Transformation|GetWorldScale (Variables|Default|GetScreenGuide))) false false))
    (:then_1
      (Transformation|SetWorldScale3D _rb_pb "0.100000,0.100000,0.100000")
      (Transformation|AddLocalOffset _rb_pb (/ (Math|Vector|MakeVector 0.0 _y_2 (* _z_2 -1.0)) (Transformation|GetWorldScale (Variables|Default|GetScreenGuide))) false false))
    (:then_2
      (Transformation|SetWorldScale3D _lt_pc "0.100000,0.100000,0.100000")
      (Transformation|AddLocalOffset _lt_pc (/ (Math|Vector|MakeVector 0.0 (* _y_3 -1.0) _z_3) (Transformation|GetWorldScale (Variables|Default|GetScreenGuide))) false false))))

(fn GetCornerPoints
  (return (Transformation|GetWorldLocation (Variables|Default|GetLB_pa)) (Transformation|GetWorldLocation (Variables|Default|GetRB_pb)) (Transformation|GetWorldLocation (Variables|Default|GetLT_pc))))